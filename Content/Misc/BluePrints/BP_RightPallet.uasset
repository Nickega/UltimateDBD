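; BP_RightPallet is a right-side pallet toggled by the D key, with input enabled for player 0 at BeginPlay.
; PalletRight moves PalletStatus between 0 and 2 through a transitional 1, setting PalletAnim and using delays to time each change; presses during transition are ignored.
; While IsPalletD is true in state 2, a looping Delay accumulates PalletTime until the toggle back clears the flag.
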(event Custom|PalletRight
  (if (== (Variables|Default|GetPalletStatus) 2)
    (Variables|Default|SetPalletAnim true)
    (Variables|Default|SetPalletStatus 1)
    (Utilities|FlowControl|Delay 0.1)
    (Variables|Default|SetIsPalletD false)
    (Utilities|FlowControl|Delay 1.01)
    (Variables|Default|SetPalletStatus 0)
    (elif (== (Variables|Default|GetPalletStatus) 0)
      (Variables|Default|SetPalletAnim true)
      (Variables|Default|SetPalletStatus 1)
      (Utilities|FlowControl|Delay 1.01)
      (Variables|Default|SetPalletStatus 2)
      (Variables|Default|SetIsPalletD true)
      (Utilities|FlowControl|Delay 0.1 :!label _label)
      (if (Variables|Default|GetIsPalletD)
        (Variables|Default|SetPalletTime (+ (Variables|Default|GetPalletTime) 0.1))
        (goto _label)))))

(event EventBeginPlay
  (Input|EnableInput (Game|GetPlayerController 0)))

(event Collision|EventActorBeginOverlap
  (params (OtherActor :type Actor%20Object%20Reference)))

(event EventTick
  (params (DeltaSeconds :type Float%20%28single-precision%29)))

(event Input|KeyboardEvents|D
  (params (Key :type Key%20Structure :default "None"))
  (:Pressed
    (CallFunction|PalletRight)))

(fn ConstructionScript)