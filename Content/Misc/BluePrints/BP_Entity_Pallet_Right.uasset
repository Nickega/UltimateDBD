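; BP_Entity_Pallet_Right is an actor for a right-side pallet that rises in small steps during a timed window.
; BeginPlay starts an endless Delay loop that polls RPalletRef every tenth of a second instead of using Tick.
; While that reference's PalletTime is within the window and IsPalletD is true, the actor offsets itself upward without sweeping.
; Nothing in this graph moves it back down.
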(event EventBeginPlay
  (bind _rpallet_ref (Variables|Default|GetRPallet%20Ref))
  (Utilities|FlowControl|Delay 0.1 :!label _label)
  (if (>= (Variables|/Game/Misc/BluePrints/BP_RightPallet.BP_RightPallet_C|GetPalletTime _rpallet_ref) 1e+01)
    (if (<= (Variables|/Game/Misc/BluePrints/BP_RightPallet.BP_RightPallet_C|GetPalletTime _rpallet_ref) 6e+01)
      (if (Variables|/Game/Misc/BluePrints/BP_RightPallet.BP_RightPallet_C|GetIsPalletD _rpallet_ref)
        (Transformation|AddActorWorldOffset "0.000000,0.000000,0.500000")
        (goto _label)
        (else
          (goto _label)))
      (else
        (goto _label)))
    (else
      (goto _label))))

(event Collision|EventActorBeginOverlap
  (params (OtherActor :type Actor%20Object%20Reference)))

(event EventTick
  (params (DeltaSeconds :type Float%20%28single-precision%29)))

(fn ConstructionScript)