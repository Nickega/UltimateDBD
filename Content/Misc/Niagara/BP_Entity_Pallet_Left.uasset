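; BP_Entity_Pallet_Left is an actor that creeps upward in the world based on left-pallet state held by the player character.
; Each Tick it casts player 0 to BP_FirstPersonCharacter and reads PalletL and the PalletLD flag.
; While PalletL is within a fixed range and PalletLD is true, it adds a small Z offset without sweep.
; The step is per frame, so its speed depends on frame rate.
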(event EventBeginPlay)

(event Collision|EventActorBeginOverlap
  (params (OtherActor :type Actor%20Object%20Reference)))

(event EventTick
  (params (DeltaSeconds :type Float%20%28single-precision%29))
  (bind _asbp_first_person_character (Utilities|Casting|CastToBP_FirstPersonCharacter (Game|GetPlayerCharacter 0)))
  (if (>= (Variables|/Game/FirstPerson/Blueprints/BP_FirstPersonCharacter.BP_FirstPersonCharacter_C|GetPalletL _asbp_first_person_character) 1e+01)
    (if (<= (Variables|/Game/FirstPerson/Blueprints/BP_FirstPersonCharacter.BP_FirstPersonCharacter_C|GetPalletL _asbp_first_person_character) 6e+01)
      (if (Variables|/Game/FirstPerson/Blueprints/BP_FirstPersonCharacter.BP_FirstPersonCharacter_C|GetPalletLD _asbp_first_person_character)
        (Transformation|AddActorWorldOffset "0.000000,0.000000,0.060000")))))

(fn ConstructionScript)