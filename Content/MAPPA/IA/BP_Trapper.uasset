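; BP_Trapper is the Trapper enemy AI, teleporting to attack one of five generators or an office side after a cooldown.
; A delay-and-random-roll loop almost always picks generators, targeting only partly charged ones via chained re-rolled checks.
; Rare office attacks check that side's pallet after a pause; the health check is hardcoded, so failure only prints "INJURED".
; Completed attacks teleport it to the world origin and restart the cooldown.
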(event EventBeginPlay
  (bind _returnvalue (Math|Random|RandomIntegerinRange 1 5))
  ;[0 0 0] Trapper AI
  ;;[0.07292 0.07292 0.07292] Cooldown
  (Utilities|FlowControl|Delay 15.0 :!label _label)
  (Utilities|FlowControl|Delay 2.0 :!label _label_2)
  ;;[0.08854 0.08854 0.08854] Attack RNG
  (if (> (Math|Random|RandomIntegerinRange 0 100) 65)
    (if (> (Math|Random|RandomIntegerinRange 0 100) 0) :!label _label_3
      ;;[0.07812 0.07812 0.07812] Gen Attack
      (if (== _returnvalue 1) :!label _label_4
        (if (> (Variables|/Game/Cameras/UMG_Tablet.UMG_Tablet_C|GetGenCharge1 (Variables|Default|GetGenCharge)) 0.0)
          (if (< (Variables|/Game/Cameras/UMG_Tablet.UMG_Tablet_C|GetGenCharge1 (Variables|Default|GetGenCharge)) 1.0)
            (Transformation|Teleport "30815.000000,504.000000,788.000000" "0, 0, 0")
            (Development|PrintText "GEN1" true true "(R=0.000000,G=0.660000,B=1.000000,A=1.000000)" 5.0)
            (else
              (goto _label)))
          (else
            (goto _label_3)))
        (elif (== _returnvalue 2)
          (if (> (Variables|/Game/Cameras/UMG_Tablet.UMG_Tablet_C|GetGenCharge2 (Variables|Default|GetGenCharge)) 0.0)
            (if (< (Variables|/Game/Cameras/UMG_Tablet.UMG_Tablet_C|GetGenCharge2 (Variables|Default|GetGenCharge)) 1.0)
              (Transformation|Teleport "34230.000000,-7614.000000,788.000000" "0, 0, 0")
              (Development|PrintText "GEN2" true true "(R=0.000000,G=0.660000,B=1.000000,A=1.000000)" 5.0)
              (else
                (goto _label)))
            (else
              (goto _label_3)))
          (elif (== _returnvalue 3)
            (if (> (Variables|/Game/Cameras/UMG_Tablet.UMG_Tablet_C|GetGenCharge3 (Variables|Default|GetGenCharge)) 0.0)
              (if (< (Variables|/Game/Cameras/UMG_Tablet.UMG_Tablet_C|GetGenCharge3 (Variables|Default|GetGenCharge)) 1.0)
                (Transformation|Teleport "37627.000000,-7764.000000,788.000000" "0.000000,529.999996,0.000000")
                (Development|PrintText "GEN3" true true "(R=0.000000,G=0.660000,B=1.000000,A=1.000000)" 5.0)
                (else
                  (goto _label)))
              (else
                (goto _label_3)))
            (elif (== _returnvalue 4)
              (if (> (Variables|/Game/Cameras/UMG_Tablet.UMG_Tablet_C|GetGenCharge4 (Variables|Default|GetGenCharge)) 0.0)
                (if (< (Variables|/Game/Cameras/UMG_Tablet.UMG_Tablet_C|GetGenCharge4 (Variables|Default|GetGenCharge)) 1.0)
                  (Transformation|Teleport "37552.000000,-795.000000,788.000000" "0.000000,799.999994,0.000000")
                  (Development|PrintText "GEN4" true true "(R=0.000000,G=0.660000,B=1.000000,A=1.000000)" 5.0)
                  (else
                    (goto _label)))
                (else
                  (goto _label_3)))
              (elif (== _returnvalue 5)
                (if (> (Variables|/Game/Cameras/UMG_Tablet.UMG_Tablet_C|GetGenCharge5 (Variables|Default|GetGenCharge)) 0.0)
                  (if (< (Variables|/Game/Cameras/UMG_Tablet.UMG_Tablet_C|GetGenCharge5 (Variables|Default|GetGenCharge)) 1.0)
                    (Transformation|Teleport "37326.000000,-3853.000000,1260.000000" "0.000000,979.999993,0.000000")
                    (Development|PrintText "GEN5" true true "(R=0.000000,G=0.660000,B=1.000000,A=1.000000)" 5.0)
                    (else
                      (goto _label)))
                  (else
                    (goto _label_3)))
                (else
                  (goto _label_4)))))))
      (Utilities|FlowControl|Delay 5.0)
      ;;[0.07812 0.07812 0.07812] TP Fuori Mappa
      (Transformation|Teleport "0, 0, 0" "0, 0, 0" :!label _label_5)
      (goto _label)
      (else
        ;;[0.1042 0.1042 0.1042] Office Attack
        ;;;[0.1979 0.1979 0.1979] Pallet Choice
        (if (== (Math|Random|RandomIntegerinRange 0 1) 1)
          (Transformation|Teleport "26997.000000,-3546.000000,788.000000" "0.000000,419.999997,0.000000")
          (Development|PrintText "SONO A DESTRA" true true "(R=0.000000,G=0.660000,B=1.000000,A=1.000000)" 5.0)
          (Utilities|FlowControl|Delay 5.0)
          (if (Variables|/Game/Misc/BluePrints/BP_RightPallet.BP_RightPallet_C|GetIsPalletD (Variables|Default|GetRPallet_Ref))
            (goto _label_5)
            (else
              _))
          (else
            (Transformation|Teleport "26987.000000,-4961.000000,788.000000" "0.000000,269.999998,0.000000")
            (Development|PrintText "SONO A SINISTRA" true true "(R=0.000000,G=0.660000,B=1.000000,A=1.000000)" 5.0)
            (Utilities|FlowControl|Delay 5.0)
            (if (Variables|/Game/Misc/BluePrints/BP_LeftPallet.BP_LeftPallet_C|GetIsPalletD (Variables|Default|GetLPallet_Ref))
              (goto _label_5)
              (else
                _))))
        ;;;[0.2865 0.2865 0.2865] Healt State Control
        (if false
          (Development|PrintText "DEAD")
          (else
            (Development|PrintText "INJURED" true true "(R=0.000000,G=0.660000,B=1.000000,A=1.000000)" 5.0)
            (goto _label_5)))))
    (else
      (goto _label_2))))

(fn ConstructionScript)